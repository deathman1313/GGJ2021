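; Radar Blueprint that holds a ClosestPart position, apparently to track the part nearest the player.
; CheckNearest stores a candidate position when it lies closer to the player pawn than to the stored ClosestPart, rather than comparing both positions' distances to the player.
; ResetNearest sets ClosestPart to a far-off sentinel position.
; The event graph is empty, so both functions rely on external callers.
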(event EventBeginPlay)

(event EventTick
  (params (DeltaSeconds :type Float%20%28single-precision%29)))

(fn CheckNearest
  (params (Inputs :type Vector))
  (bind _asbp_player_character (Utilities|Casting|CastToBP_PlayerCharacter (Game|Player|GetPlayerPawn 0)))
  (if (< (Math|Vector|Distance(Vector) Inputs (Transformation|GetActorLocation _asbp_player_character)) (Math|Vector|Distance(Vector) Inputs (Variables|Default|GetClosestPart)))
    (bind _output_get (Variables|Default|SetClosestPart Inputs))))

(fn ResetNearest
  (Variables|Default|SetClosestPart "10000.000000,10000.000000,10000.000000"))