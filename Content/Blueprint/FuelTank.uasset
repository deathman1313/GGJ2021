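; Fuel tank pickup actor that permanently expands the player's fuel capacity when interacted with.
; On Interact, it adds FuelIncrease to both the maximum and current fuel on the player character's Fuel component.
; It then prints the new fuel totals, tells the player's Radar to reset its nearest target and destroys itself.
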(event EventBeginPlay)

(event Collision|EventActorBeginOverlap
  (params (OtherActor :type Actor%20Object%20Reference)))

(event EventTick
  (params (DeltaSeconds :type Float%20%28single-precision%29)))

(event EventInteract
  (bind _asbp_player_character (Utilities|Casting|CastToBP_PlayerCharacter (Game|Player|GetPlayerPawn 0)))
  (bind _output_get (Variables|/Game/Blueprint/Fuel.Fuel_C|SetmaxFuel (Variables|/Game/Blueprint/BP_PlayerCharacter.BP_PlayerCharacter_C|GetFuel _asbp_player_character) (+ (Variables|/Game/Blueprint/Fuel.Fuel_C|GetmaxFuel (Variables|/Game/Blueprint/BP_PlayerCharacter.BP_PlayerCharacter_C|GetFuel _asbp_player_character)) (Variables|Default|GetFuelIncrease))))
  (bind _output_get_2 (Variables|/Game/Blueprint/Fuel.Fuel_C|SetfuelAmount (Variables|/Game/Blueprint/BP_PlayerCharacter.BP_PlayerCharacter_C|GetFuel _asbp_player_character) (+ (Variables|/Game/Blueprint/Fuel.Fuel_C|GetfuelAmount (Variables|/Game/Blueprint/BP_PlayerCharacter.BP_PlayerCharacter_C|GetFuel _asbp_player_character)) (Variables|Default|GetFuelIncrease))))
  (Development|PrintString (Utilities|String|Append (Utilities|String|ToString(Float) _output_get_2) "/" (Utilities|String|ToString(Float) _output_get)))
  (Default|ResetNearest (Variables|/Game/Blueprint/BP_PlayerCharacter.BP_PlayerCharacter_C|GetRadar _asbp_player_character))
  (Actor|DestroyActor))

(fn ConstructionScript)