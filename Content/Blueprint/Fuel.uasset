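; Fuel Blueprint that drains the player character's fuel while it moves and disables its movement when the tank runs out.
; Each tick checks the pawn's velocity, lowers FuelAmount by a frame-time-scaled rate and evaluates the remaining percentage.
; A DoOnce plays a low-fuel sound at the player below the threshold, resetting when a moving check finds fuel above it.
; While stationary with Refueling set, fuel refills faster than it drains.
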(event EventBeginPlay)

(event EventTick
  (params (DeltaSeconds :type Float%20%28single-precision%29))
  (bind _returnvalue (Game|Player|GetPlayerPawn 0))
  (bind _ismoving (CallFunction|CheckMovement))
  (if _ismoving
    (Variables|Default|SetfuelAmount (- (Variables|Default|GetfuelAmount) (* (Variables|Default|GetfuelDrainRate) (Utilities|Time|GetWorldDeltaSeconds))))
    (bind (_isempty _percentleft) (CallFunction|CheckEmpty))
    (if _isempty
      (bind _asbp_player_character (Utilities|Casting|CastToBP_PlayerCharacter _returnvalue))
      (Pawn|Components|CharacterMovement|DisableMovement (Variables|/Script/Engine.Character|GetCharacterMovement _asbp_player_character))
      (elif (< _percentleft (Variables|Default|GetLowFuelPercent))
        (Utilities|FlowControl|DoOnce false :!label _label
          (:Completed
            (bind _asbp_player_character_2 (Utilities|Casting|CastToBP_PlayerCharacter _returnvalue))
            (Audio|PlaySoundatLocation "/Game/Sounds/FuelLow.FuelLow" (Transformation|GetActorLocation _asbp_player_character_2) "0, 0, 0" 1.0 1.0 0.0 0 0 0)))
        (else
          (goto _label Reset))))
    (elif (Variables|Default|GetRefueling)
      (CallFunction|Refuel))))

(fn CheckEmpty
  (bind _fuelamount (Variables|Default|GetfuelAmount))
  (return (< _fuelamount 0.0) (* (/ _fuelamount (Variables|Default|GetmaxFuel)) 1e+02)))

(fn Refuel
  (if (< (Variables|Default|GetfuelAmount) (Variables|Default|GetmaxFuel))
    (bind _output_get (Variables|Default|SetfuelAmount (+ (* (* (Variables|Default|GetfuelDrainRate) (Utilities|Time|GetWorldDeltaSeconds)) 2.5) (Variables|Default|GetfuelAmount))))))

(fn CheckMovement
  (bind _asbp_player_character (Utilities|Casting|CastToBP_PlayerCharacter (Game|Player|GetPlayerPawn 0)))
  (return (Math|Vector|NotEqual(Vector) (Variables|/Script/Engine.MovementComponent|GetVelocity (Variables|/Script/Engine.Character|GetCharacterMovement _asbp_player_character)) "0, 0, 0" 0.0001)))