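; MemoryDisk is an interactable pickup that unlocks the player's next locked memory and then destroys itself.
; It registers in the game mode's PartsList on BeginPlay, then on Interact removes itself and resets the player Radar's nearest target.
; A counting loop over the player's Memories unlocks the first locked entry.
; When that count reaches the array's length, it calls Reveal on the game mode's Bff.
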(event EventBeginPlay
  (bind _asbp_game_mode_base (Utilities|Casting|CastToBP_GameModeBase (Game|GetGameMode)))
  (Utilities|Array|Add (Variables|/Game/Blueprint/BP_GameModeBase.BP_GameModeBase_C|GetPartsList _asbp_game_mode_base) self))

(event Collision|EventActorBeginOverlap
  (params (OtherActor :type Actor%20Object%20Reference)))

(event EventTick
  (params (DeltaSeconds :type Float%20%28single-precision%29)))

(event EventInteract
  (bind _asbp_game_mode_base (Utilities|Casting|CastToBP_GameModeBase (Game|GetGameMode)))
  (bind _asbp_player_character (Utilities|Casting|CastToBP_PlayerCharacter (Game|Player|GetPlayerPawn 0)))
  ;[1 1 1] Loop Memories and set first locked
  (Default|ResetNearest (Variables|/Game/Blueprint/BP_PlayerCharacter.BP_PlayerCharacter_C|GetRadar _asbp_player_character))
  (Utilities|Array|RemoveItem (Variables|/Game/Blueprint/BP_GameModeBase.BP_GameModeBase_C|GetPartsList _asbp_game_mode_base) self)
  (bind (_array_element _array_index) (Utilities|Array|ForEachLoopwithBreak (Variables|/Game/Blueprint/BP_PlayerCharacter.BP_PlayerCharacter_C|GetMemories _asbp_player_character) :!label _label)
    (:LoopBody
      (bind _result (Math|Integer|IncrementInt (Variables|Default|GetUnlockAmount))
        (:%20%20
          (bind _output_get (Variables|Default|SetUnlockAmount _result))
          (if (not (.Unlocked (Utilities|Struct|BreakStruct_Memory _array_element)))
            (Utilities|Array|SetArrayElem (Variables|/Game/Blueprint/BP_PlayerCharacter.BP_PlayerCharacter_C|GetMemories _asbp_player_character) _array_index (Utilities|Struct|MakeStruct_Memory (.name (Utilities|Array|Get(acopy) (Variables|/Game/Blueprint/BP_PlayerCharacter.BP_PlayerCharacter_C|GetMemories _asbp_player_character) _array_index)) true (.text (Utilities|Array|Get(acopy) (Variables|/Game/Blueprint/BP_PlayerCharacter.BP_PlayerCharacter_C|GetMemories _asbp_player_character) _array_index))))
            (goto _label Break)))))
    (:Completed
      (bind _asbp_player_character_2 (Utilities|Casting|CastToBP_PlayerCharacter (Game|Player|GetPlayerPawn 0)))
      (Utilities|FlowControl|Sequence
        (:then_0
          (Math|Integer|CompareInt _output_get (Utilities|Array|Length (Variables|/Game/Blueprint/BP_PlayerCharacter.BP_PlayerCharacter_C|GetMemories _asbp_player_character_2))
            (:==
              (bind _asbp_game_mode_base_2 (Utilities|Casting|CastToBP_GameModeBase (Game|GetGameMode)))
              (Default|Reveal (Variables|/Game/Blueprint/BP_GameModeBase.BP_GameModeBase_C|GetBff _asbp_game_mode_base_2)))))
        (:then_1
          (Actor|DestroyActor))))))

(fn ConstructionScript)